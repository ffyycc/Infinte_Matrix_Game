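; BP_Tunnel is an endless-runner tunnel segment with a spinning holed wall for the player to pass through.
; Reaching the trigger zone adds score, has NewestTunnel spawn another segment and destroys this one.
; Hitting the wall costs score and HP; at zero HP it refunds that score penalty, marks death and shows restart.
; RandomizeWall, not called here, picks a random hole mesh from the player's HP band and randomizes its roll.
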(event `self.ReceiveTick`
  (params (DeltaSeconds :type "Float (single-precision)"))
  (`SceneComponent.K2_AddLocalRotation` (`self.WallMesh`) (`KismetMathLibrary.MakeRotator` (* DeltaSeconds (`self.RotateSpeed`))) false false))

(event `self.TriggerZone.OnComponentBeginOverlap`
  (params (OverlappedComponent :type "PrimitiveComponent Object Reference") (OtherActor :type "Actor Object Reference") (OtherComp :type "PrimitiveComponent Object Reference") (OtherBodyIndex :type Integer) (bFromSweep :type Boolean) (SweepResult :type "HitResult Structure (by ref)"))
  (bind _asbp_player (cast `/Game/InfiniteMatrix/Blueprints/BP_Player` OtherActor))
  (set `/Game/InfiniteMatrix/Blueprints/BP_Player.Score` (+ (`/Game/InfiniteMatrix/Blueprints/BP_Player.Score` _asbp_player) 5) _asbp_player)
  (`/Game/InfiniteMatrix/Blueprints/BP_TunnelSpawner.SpawnTunnelAtSpawnPoint` (`self.Newest Tunnel`))
  (`self.K2_DestroyActor`))

(event `self.WallMesh.OnComponentBeginOverlap`
  (params (OverlappedComponent :type "PrimitiveComponent Object Reference") (OtherActor :type "Actor Object Reference") (OtherComp :type "PrimitiveComponent Object Reference") (OtherBodyIndex :type Integer) (bFromSweep :type Boolean) (SweepResult :type "HitResult Structure (by ref)"))
  (bind _asbp_player (cast `/Game/InfiniteMatrix/Blueprints/BP_Player` OtherActor))
  (set `/Game/InfiniteMatrix/Blueprints/BP_Player.Score` (- (`/Game/InfiniteMatrix/Blueprints/BP_Player.Score` _asbp_player) 5) _asbp_player)
  (bind _output_get (set `/Game/InfiniteMatrix/Blueprints/BP_Player.HP` (- (`/Game/InfiniteMatrix/Blueprints/BP_Player.HP` _asbp_player) 20) _asbp_player))
  (if (<= _output_get 0)
    (bind _asbp_player_2 (cast `/Game/InfiniteMatrix/Blueprints/BP_Player` _asbp_player))
    (set `/Game/InfiniteMatrix/Blueprints/BP_Player.Score` (+ (`/Game/InfiniteMatrix/Blueprints/BP_Player.Score` _asbp_player_2) 5) _asbp_player_2)
    (set `/Game/InfiniteMatrix/Blueprints/BP_Player.IsDead` true _asbp_player)
    (`/Game/InfiniteMatrix/Blueprints/BP_Player.DisplayRestart` _asbp_player)))

(fn `RandomizeWall`
  (bind _asbp_player (cast `/Game/InfiniteMatrix/Blueprints/BP_Player` (`GameplayStatics.GetPlayerPawn` 0)))
  (bind _hp (`/Game/InfiniteMatrix/Blueprints/BP_Player.HP` _asbp_player))
  (if (> _hp 80)
    (`StaticMeshComponent.SetStaticMesh` (`self.WallMesh`) (select `int` (`KismetMathLibrary.RandomIntegerInRange` 0 3) :`0` "/Game/InfiniteMatrix/Meshes/SM_Hole_01.SM_Hole_01" :`1` "/Game/InfiniteMatrix/Meshes/SM_Hole_02.SM_Hole_02" :`2` "/Game/InfiniteMatrix/Meshes/SM_Hole_03.SM_Hole_03" :`3` "/Game/InfiniteMatrix/Meshes/SM_Hole_04.SM_Hole_04" :!type "StaticMesh Object Reference"))
    (`SceneComponent.K2_AddLocalRotation` (`self.WallMesh`) (`KismetMathLibrary.MakeRotator` (`KismetMathLibrary.RandomFloatInRange` 0.0 360.0)) false false)
    (elif (> _hp 60)
      (`StaticMeshComponent.SetStaticMesh` (`self.WallMesh`) (select `int` (`KismetMathLibrary.RandomIntegerInRange` 0 3) :`0` "/Game/InfiniteMatrix/Meshes/Hole_01_80.Hole_01_80" :`1` "/Game/InfiniteMatrix/Meshes/Hole_02_80.Hole_02_80" :`2` "/Game/InfiniteMatrix/Meshes/Hole_03_80.Hole_03_80" :`3` "/Game/InfiniteMatrix/Meshes/Hole_04_80.Hole_04_80" :!type "StaticMesh Object Reference"))
      (`SceneComponent.K2_AddLocalRotation` (`self.WallMesh`) (`KismetMathLibrary.MakeRotator` (`KismetMathLibrary.RandomFloatInRange` 0.0 360.0)) false false)
      (else
        (bind _hp_2 (`/Game/InfiniteMatrix/Blueprints/BP_Player.HP` _asbp_player))
        (if (> _hp_2 40)
          (`StaticMeshComponent.SetStaticMesh` (`self.WallMesh`) (select `int` (`KismetMathLibrary.RandomIntegerInRange` 0 3) :`0` "/Game/InfiniteMatrix/Meshes/Hole_01_60.Hole_01_60" :`1` "/Game/InfiniteMatrix/Meshes/Hole_02_60.Hole_02_60" :`2` "/Game/InfiniteMatrix/Meshes/Hole_03_60.Hole_03_60" :`3` "/Game/InfiniteMatrix/Meshes/Hole_04_60.Hole_04_60" :!type "StaticMesh Object Reference"))
          (`SceneComponent.K2_AddLocalRotation` (`self.WallMesh`) (`KismetMathLibrary.MakeRotator` (`KismetMathLibrary.RandomFloatInRange` 0.0 360.0)) false false)
          (elif (> _hp_2 20)
            (`StaticMeshComponent.SetStaticMesh` (`self.WallMesh`) (select `int` (`KismetMathLibrary.RandomIntegerInRange` 0 3) :`0` "/Game/InfiniteMatrix/Meshes/Hole_01_40.Hole_01_40" :`1` "/Game/InfiniteMatrix/Meshes/Hole_02_40.Hole_02_40" :`2` "/Game/InfiniteMatrix/Meshes/Hole_03_40.Hole_03_40" :`3` "/Game/InfiniteMatrix/Meshes/Hole_04_40.Hole_04_40" :!type "StaticMesh Object Reference"))
            (`SceneComponent.K2_AddLocalRotation` (`self.WallMesh`) (`KismetMathLibrary.MakeRotator` (`KismetMathLibrary.RandomFloatInRange` 0.0 360.0)) false false)
            (else
              (`StaticMeshComponent.SetStaticMesh` (`self.WallMesh`) (select `int` (`KismetMathLibrary.RandomIntegerInRange` 0 3) :`0` "/Game/InfiniteMatrix/Meshes/Hole_01_20.Hole_01_20" :`1` "/Game/InfiniteMatrix/Meshes/Hole_02_20.Hole_02_20" :`2` "/Game/InfiniteMatrix/Meshes/Hole_03_20.Hole_03_20" :`3` "/Game/InfiniteMatrix/Meshes/Hole_04_20.Hole_04_20" :!type "StaticMesh Object Reference"))
              (`SceneComponent.K2_AddLocalRotation` (`self.WallMesh`) (`KismetMathLibrary.MakeRotator` (`KismetMathLibrary.RandomFloatInRange` 0.0 360.0)) false false))))))))

(fn `UserConstructionScript`)