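; Projectile actor, by its name a shot, that destroys enemies and awards score.
; When its Sphere overlaps an EnemyNew, it destroys that enemy and adds points to the player BP_Player's Score, without destroying itself.
; Tick accumulates delta time into Velocity, which acts as a lifetime timer that destroys the actor at a threshold; the graphs contain no movement logic.
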(event `self.ReceiveTick`
  (params (DeltaSeconds :type "Float (single-precision)"))
  (bind _output_get (set `self.velocity` (+ DeltaSeconds (`self.velocity`))))
  (if (>= _output_get 125.0)
    (`self.K2_DestroyActor`)))

(event `self.Sphere.OnComponentBeginOverlap`
  (params (OverlappedComponent :type "PrimitiveComponent Object Reference") (OtherActor :type "Actor Object Reference") (OtherComp :type "PrimitiveComponent Object Reference") (OtherBodyIndex :type Integer) (bFromSweep :type Boolean) (SweepResult :type "HitResult Structure (by ref)"))
  (bind _asenemy_new (cast `/Game/InfiniteMatrix/Blueprints/EnemyNew` OtherActor))
  (`self.K2_DestroyActor` _asenemy_new)
  (bind _asbp_player (cast `/Game/InfiniteMatrix/Blueprints/BP_Player` (`GameplayStatics.GetPlayerPawn` 0)))
  (set `/Game/InfiniteMatrix/Blueprints/BP_Player.Score` (+ (`/Game/InfiniteMatrix/Blueprints/BP_Player.Score` _asbp_player) 5) _asbp_player))

(fn `UserConstructionScript`)