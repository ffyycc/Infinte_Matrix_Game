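; EnemyNew is an enemy actor that damages the player on contact and destroys itself.
; A hit on its Enemy component casts the other actor to BP_Player and subtracts a fixed amount from that player's HP.
; When the hit would bring HP to zero or below, it clamps HP, flags the player dead and calls DisplayRestart on the player.
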(event `self.Enemy.OnComponentHit`
  (params (HitComponent :type "PrimitiveComponent Object Reference") (OtherActor :type "Actor Object Reference") (OtherComp :type "PrimitiveComponent Object Reference") (NormalImpulse :type "Vector Structure") (Hit :type "HitResult Structure (by ref)"))
  (bind _asbp_player (cast `/Game/InfiniteMatrix/Blueprints/BP_Player` OtherActor))
  (bind _returnvalue (- (`/Game/InfiniteMatrix/Blueprints/BP_Player.HP` _asbp_player) 20))
  (if (> _returnvalue 0)
    (set `/Game/InfiniteMatrix/Blueprints/BP_Player.HP` _returnvalue _asbp_player)
    (`self.K2_DestroyActor`)
    (else
      (set `/Game/InfiniteMatrix/Blueprints/BP_Player.HP` 0 _asbp_player)
      (set `/Game/InfiniteMatrix/Blueprints/BP_Player.IsDead` true _asbp_player)
      (`/Game/InfiniteMatrix/Blueprints/BP_Player.DisplayRestart` _asbp_player)
      (`self.K2_DestroyActor`))))

(fn `UserConstructionScript`)