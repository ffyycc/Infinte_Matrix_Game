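; Spawner that builds a chain of BP_Tunnel segments for an endless tunnel and populates them with pickups and enemies.
; On BeginPlay it clears existing tunnels, then spawns a few, starting at the player pawn and chaining from the newest segment's SpawnPoint.
; Each segment receives a spawner reference, randomizes its wall, and independently rolls for a HealthPack and an EnemyNew at random offsets ahead.
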(event `self.ReceiveBeginPlay`
  (`self.SpawnInitialTUnnels`))

(fn `AddHealthPack`
  (params (location :type "Vector Structure"))
  (if (== (`KismetMathLibrary.RandomIntegerInRange` 0 5) 0)
    (`|SpawnActorFromClass` "/Game/InfiniteMatrix/Blueprints/HealthPack.HealthPack_C" (`KismetMathLibrary.MakeTransform` (`KismetMathLibrary.MakeVector` (+ (.x location) (`KismetMathLibrary.RandomFloatInRange` 1250.0 1875.0)) (+ (.y location) (`KismetMathLibrary.RandomFloatInRange` -200.0 200.0)) (+ (.z location) (`KismetMathLibrary.RandomFloatInRange` -200.0 200.0))) (struct) (20.0 20.0 20.0)) "Undefined" "OverrideRootScale" null null)))

(fn `SpawnEnemy`
  (params (`enemy vector` :type "Vector Structure"))
  (if (== (`KismetMathLibrary.RandomIntegerInRange` 0 2) 0)
    (`|SpawnActorFromClass` "/Game/InfiniteMatrix/Blueprints/EnemyNew.EnemyNew_C" (`KismetMathLibrary.MakeTransform` (`KismetMathLibrary.MakeVector` (+ (.x `enemy vector`) (`KismetMathLibrary.RandomFloatInRange` 1250.0 1875.0)) (+ (.y `enemy vector`) (`KismetMathLibrary.RandomFloatInRange` -200.0 200.0)) (+ (.z `enemy vector`) (`KismetMathLibrary.RandomFloatInRange` -200.0 200.0))) (struct) (20.0 20.0 20.0)) "Undefined" "OverrideRootScale" null null)))

(fn `SpawnInitialTUnnels`
  (`|ExecutionSequence`
    (:`then_0`
      (bind _outactors (`GameplayStatics.GetAllActorsOfClass` "/Game/InfiniteMatrix/Blueprints/BP_Tunnel.BP_Tunnel_C"))
      (for _array_element _outactors
        (`self.K2_DestroyActor` _array_element)))
    (:`then_1`
      (for _ (range 3)
        (`/Engine/EditorBlueprintResources/StandardMacros.IsValid` (`self.Newest Tunnel`)
          (:`Is Valid`
            (`self.SpawnTunnelAtSpawnPoint`))
          (:`Is Not Valid`
            (`self.SpawnTUnnel` (`self.K2_GetActorLocation` (`GameplayStatics.GetPlayerPawn` 0)))))))))

(fn `SpawnTUnnel`
  (params (SpawnLocation :type "Vector Structure"))
  (locals (NewLocalVar_0 :type "/Game/InfiniteMatrix/Blueprints/BP_Tunnel Object Reference") (NewLocalVar_1 :type "/Game/InfiniteMatrix/Blueprints/BP_Tunnel Object Reference") (NewLocalVar_2 :type "/Game/InfiniteMatrix/Blueprints/BP_TunnelSpawner Object Reference") (NewLocalVar_3 :type "/Game/InfiniteMatrix/Blueprints/BP_Tunnel Object Reference") (NewLocalVar_4 :type "/Game/InfiniteMatrix/Blueprints/BP_TunnelSpawner Object Reference"))
  (bind _returnvalue (`|SpawnActorFromClass` "/Game/InfiniteMatrix/Blueprints/BP_Tunnel.BP_Tunnel_C" (`KismetMathLibrary.MakeTransform` SpawnLocation) "Undefined" "OverrideRootScale" null null))
  (bind _output_get (set `self.Newest Tunnel` _returnvalue))
  (set `/Game/InfiniteMatrix/Blueprints/BP_Tunnel.Newest Tunnel` self _output_get)
  (`/Game/InfiniteMatrix/Blueprints/BP_Tunnel.RandomizeWall` _output_get)
  (`self.AddHealthPack` SpawnLocation)
  (`self.SpawnEnemy` SpawnLocation))

(fn `SpawnTunnelAtSpawnPoint`
  (`self.SpawnTUnnel` (`SceneComponent.K2_GetComponentLocation` (`/Game/InfiniteMatrix/Blueprints/BP_Tunnel.SpawnPoint` (`self.Newest Tunnel`)))))

(fn `UserConstructionScript`)